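; Passcode door Blueprint that opens a Numpad widget on E and destroys itself when OpenDoor is called.
; Trigger overlaps use FlipFlops, alternating between toggling input for BP_Topdown_MC and toggling the Press prompt, rather than doing both each time.
; E alternates between showing the numpad with cursor and UI input, and clearing all widgets to restore game-only input.
; Exit's input-disabling branch shares that cleanup.
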(event `self.Door_trigger.OnComponentBeginOverlap`
  (params (OverlappedComponent :type "PrimitiveComponent Object Reference") (OtherActor :type "Actor Object Reference") (OtherComp :type "PrimitiveComponent Object Reference") (OtherBodyIndex :type Integer) (bFromSweep :type Boolean) (SweepResult :type "HitResult Structure (by ref)"))
  (`/Engine/EditorBlueprintResources/StandardMacros.FlipFlop`
    (:`A`
      (cast `/Game/Material/Charactor/BP_Topdown_MC` OtherActor)
      (`self.EnableInput` (`GameplayStatics.GetPlayerController` 0)))
    (:`B`
      (`SceneComponent.SetVisibility` (`self.Press`) true false))))

(event `self.Door_trigger.OnComponentEndOverlap`
  (params (OverlappedComponent :type "PrimitiveComponent Object Reference") (OtherActor :type "Actor Object Reference") (OtherComp :type "PrimitiveComponent Object Reference") (OtherBodyIndex :type Integer))
  (bind _returnvalue (`GameplayStatics.GetPlayerController` 0))
  (`/Engine/EditorBlueprintResources/StandardMacros.FlipFlop`
    (:`A`
      (cast `/Game/Material/Charactor/BP_Topdown_MC` OtherActor)
      (`self.DisableInput` (`GameplayStatics.GetPlayerController` 0))
      (`WidgetLayoutLibrary.RemoveAllWidgets` :!label _label)
      (`WidgetBlueprintLibrary.SetInputMode_GameOnly` _returnvalue)
      (set `PlayerController.bShowMouseCursor` false _returnvalue))
    (:`B`
      (`SceneComponent.SetVisibility` (`self.Press`) false false))))

(event `Key|E`
  (params (Key :type "Key Structure"))
  (bind _returnvalue (`GameplayStatics.GetPlayerController` 0))
  (:`Pressed`
    (`/Engine/EditorBlueprintResources/StandardMacros.FlipFlop`
      (:`A`
        (bind _returnvalue_2 (`|CreateWidget` "/Game/UI/Numpad.Numpad_C"))
        (`UserWidget.AddToViewport` _returnvalue_2 0)
        (`WidgetBlueprintLibrary.SetInputMode_GameAndUIEx` _returnvalue _returnvalue_2)
        (set `PlayerController.bShowMouseCursor` true _returnvalue))
      (:`B`
        (goto _label)))))

(event `OpenDoor`
  (`WidgetLayoutLibrary.RemoveAllWidgets`)
  (`self.K2_DestroyActor`))

(fn `UserConstructionScript`)